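; Enemy Blueprint that chases the player and can be killed by damage.
; PawnSensing sets a seen flag on spotting any pawn, then FollowPlayer issues an AI MoveTo toward player character 0; the flag is never cleared here.
; TakeDamage subtracts from current HP, clamped between zero and max, and destroys the actor when it reaches zero.
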(event `self.PawnSensing.OnSeePawn`
  (params (Pawn :type "Pawn Object Reference"))
  (set `self.isSeeingPlayer` true)
  (`self.FollowPlayer`))

(event `FollowPlayer`
  (if (`self.isSeeingPlayer`)
    (`|AIMoveTo` self (0.0 0.0 0.0) (`GameplayStatics.GetPlayerCharacter` 0))))

(event `Take Damage`
  (params (`Damage Taken` :type "Float (double-precision)"))
  (bind _output_get (set `self.CurrentHP` (`KismetMathLibrary.FClamp` (- (`self.CurrentHP`) `Damage Taken`) 0.0 (`self.MaxHP`))))
  (if (<= _output_get 0.0)
    (`self.K2_DestroyActor`)))

(fn `UserConstructionScript`)